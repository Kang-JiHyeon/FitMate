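; BP_Player is a player Blueprint with a scene capture of its own mesh and a set of cosmetic hat and Piero components.
; BeginPlay sets the capture to HDR scene color, captures once, then restricts it to the Mesh, and adds the WBP_PlayerUI widget to the viewport.
; It also gathers the cosmetics into an array, which OnMeguminsHat indexes to make the Megumin hat visible.
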(event EventBeginPlay
  (bind _scenecapturecomponent2d (Variables|Default|GetSceneCaptureComponent2D))
  (Variables|/Script/Engine.SceneCaptureComponent|SetCaptureSource _scenecapturecomponent2d "SCS_SceneColorHDR")
  (Rendering|SceneCapture|CaptureScene _scenecapturecomponent2d :!class /Script/Engine.SceneCaptureComponent2D)
  (Rendering|SceneCapture|ShowOnlyComponent _scenecapturecomponent2d (Variables|Character|GetMesh))
  (bind _returnvalue (UserInterface|CreateWidget "/Game/CSW/UI/WBP_PlayerUI.WBP_PlayerUI_C"))
  (UserInterface|Viewport|AddtoViewport _returnvalue 0)
  (Variables|Default|SetArray (Utilities|Array|MakeArray (Variables|Default|Getmegumins_hat) (Variables|Default|Getrupy_hat_1) (Variables|Default|Getrupy_hat_2) (Variables|Default|Getpiero1) (Variables|Default|Getpiero2) (Variables|Default|Getpiero3) (Variables|Default|Getpiero4) (Variables|Default|Getpiero5) (Variables|Default|Getpiero6) (Variables|Default|Getpiero7))))

(event Collision|EventActorBeginOverlap
  (params (OtherActor :type Actor%20Object%20Reference)))

(event EventTick
  (params (DeltaSeconds :type Float%20%28single-precision%29)))

(fn ConstructionScript)

(fn OnMeguminsHat
  (Rendering|SetVisibility (Utilities|Array|Get(acopy) (Variables|Default|GetArray)) true false))